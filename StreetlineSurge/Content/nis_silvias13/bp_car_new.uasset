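; A drivable car Blueprint that uses Enhanced Input and a vehicle movement component.
; On possession it prints a debug string and adds the car input mapping context for player 0.
; Brake and steer actions feed the movement component, but the throttle action is unwired.
; Tick instead forces full throttle every frame and prints the mesh's physics linear velocity for debugging.
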(event Input|EnhancedActionEvents|EnhancedInputActionia_brake
  (params (ActionValue :type Float%20%28double-precision%29) (ElapsedSeconds :type Float%20%28double-precision%29) (TriggeredSeconds :type Float%20%28double-precision%29) (InputAction :type Input%20Action%20Object%20Reference :default "/Game/nis_silvias13/ia_brake.ia_brake"))
  (Class|ChaosVehicleMovementComponent|SetBrakeInput (Variables|Default|GetVehicleMovementComponent) ActionValue))

(event Input|EnhancedActionEvents|EnhancedInputActionia_steer
  (params (ActionValue :type Float%20%28double-precision%29) (ElapsedSeconds :type Float%20%28double-precision%29) (TriggeredSeconds :type Float%20%28double-precision%29) (InputAction :type Input%20Action%20Object%20Reference :default "/Game/nis_silvias13/ia_steer.ia_steer"))
  (Class|ChaosVehicleMovementComponent|SetSteeringInput (Variables|Default|GetVehicleMovementComponent) ActionValue))

(event Input|EnhancedActionEvents|EnhancedInputActionia_throttle
  (params (ActionValue :type Float%20%28double-precision%29) (ElapsedSeconds :type Float%20%28double-precision%29) (TriggeredSeconds :type Float%20%28double-precision%29) (InputAction :type Input%20Action%20Object%20Reference :default "/Game/nis_silvias13/ia_throttle.ia_throttle")))

(event EventBeginPlay)

(event Collision|EventActorBeginOverlap
  (params (OtherActor :type Actor%20Object%20Reference)))

(event EventPossessed
  (params (NewController :type Controller%20Object%20Reference))
  (Development|PrintString "tung tung")
  (Input|AddMappingContext (PlayerController|LocalPlayerSubsystems|GetEnhancedInputLocalPlayerSubsystem (Game|GetPlayerController 0)) "/Game/nis_silvias13/imc_car.imc_car" 0 "(bIgnoreAllPressedKeysUntilRelease=True,bForceImmediately=False,bNotifyUserSettings=False)"))

(event EventTick
  (params (DeltaSeconds :type Float%20%28single-precision%29))
  (Class|ChaosVehicleMovementComponent|SetThrottleInput (Variables|Default|GetVehicleMovementComponent) 1.0)
  (bind _returnvalue (Physics|GetPhysicsLinearVelocity (Variables|Character|GetMesh) "None"))
  (Development|PrintString (Utilities|String|ToString(Vector) _returnvalue)))

(fn ConstructionScript)